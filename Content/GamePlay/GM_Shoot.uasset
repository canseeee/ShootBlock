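; GM_Shoot is a game mode that runs a timed match and spawns player characters.
; PostLogin collects player controllers, finds the ActorBigTime clock and starts a one-second looping timer once.
; Each tick decrements EndTime onto that clock, or at zero calls EventPCEnd on every controller, without clearing the timer.
; Event_Spawn possesses either a fixed-position first-person character or a randomly placed third-person one, which gets EventAdd ten seconds later.
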(event `self.K2_PostLogin`
  (params (NewPlayer :type "PlayerController Object Reference"))
  (`|ExecutionSequence`
    (:`then_0`
      (bind _output_get (set `self.LoginPlayer` NewPlayer))
      (bind _asbp_first_person_player_controller (cast `/Game/FirstPerson/Blueprints/BP_FirstPersonPlayerController` _output_get))
      (`KismetArrayLibrary.Array_AddUnique` (`self.As PC Lobby BP`) _asbp_first_person_player_controller)
      (bind _returnvalue (`GameplayStatics.GetActorOfClass` "/Game/UMG/ActorBigTime.ActorBigTime_C"))
      (set `self.BigTime` _returnvalue)
      (`/Engine/EditorBlueprintResources/StandardMacros.DoOnce` false
        (:`Completed`
          (`KismetSystemLibrary.K2_SetTimerDelegate` (delegate `Event_Time`) 1.0 true))))))

(event `Event_End`
  (for _array_element (`self.As PC Lobby BP`)
    (`/Game/FirstPerson/Blueprints/BP_FirstPersonPlayerController.Event_PCEnd` _array_element)))

(event `Event_Time`
  (if (<= (`self.EndTime`) 0)
    (`self.Event_End`)
    (else
      (bind _output_get (set `self.EndTime` (- (`self.EndTime`) 1)))
      (`/Game/UMG/ActorBigTime.AddTime` (`self.BigTime`) _output_get))))

(event `Event_Spawn`
  (params (Condition :type Boolean) (NewParam :type "Controller Object Reference"))
  (bind _new_player (`self.New Player`))
  (set `self.New Player` NewParam)
  (if Condition
    (bind _returnvalue (`|SpawnActorFromClass` "/Game/FirstPerson/Blueprints/BP_FirstPersonCharacter.BP_FirstPersonCharacter_C" (`KismetMathLibrary.MakeTransform` (900.0 850.0 90.0)) "Undefined" "MultiplyWithRoot" _new_player null))
    (`Controller.Possess` (`self.New Player`) _returnvalue)
    (else
      (bind _returnvalue_2 (`|SpawnActorFromClass` "/Game/ThirdPerson/Blueprints/BP_ThirdPersonCharacter.BP_ThirdPersonCharacter_C" (`KismetMathLibrary.MakeTransform` (`KismetMathLibrary.MakeVector` (`KismetMathLibrary.RandomFloatInRange` 1000.0 2000.0) (`KismetMathLibrary.RandomFloatInRange` 2000.0 3000.0) 90.0)) "Undefined" "MultiplyWithRoot" _new_player null))
      (`Controller.Possess` (`self.New Player`) _returnvalue_2)
      (`KismetSystemLibrary.Delay` 10.0)
      (`/Game/ThirdPerson/Blueprints/BP_ThirdPersonCharacter.EventAdd` _returnvalue_2))))

(fn `UserConstructionScript`)