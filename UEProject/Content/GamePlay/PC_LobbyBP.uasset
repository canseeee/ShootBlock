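; Lobby player controller that creates the lobby and login widgets for the local player on BeginPlay and shows the mouse cursor.
; IsBlock and IsShoot events write their values into the GS_Lobby game state.
; Event "2" passes a check state to the lobby widget and prints a server/client debug string.
; Unwired leftover logic would host or find and join a LAN session by authority.
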(event `self.ReceiveBeginPlay`
  (`|ExecutionSequence`
    (:`then_1`
      (`self.Func_UI`))))

(event `IsBlock`
  (params (NewParam :type Boolean) (NewParam2 :type Integer))
  (bind _asgs_lobby (cast `/Game/GamePlay/GS_Lobby` (`GameplayStatics.GetGameState`)))
  (set `/Game/GamePlay/GS_Lobby.Num` NewParam2 _asgs_lobby)
  (set `/Game/GamePlay/GS_Lobby.IsBlock` NewParam _asgs_lobby))

(event `2`
  (params (NewParam :type Boolean))
  (bind _ui (`self.ui`))
  (`/Engine/EditorBlueprintResources/StandardMacros.IsValid` _ui
    (:`Is Valid`
      (`/Game/UMG/UI_Lobby.Event_ReturnCheck` _ui NewParam 0)
      (`/Engine/EditorBlueprintResources/ActorMacros.Switch Has Authority`
        (:`Authority`
          (`KismetSystemLibrary.PrintString` "s" true true (struct :`G` 0.66 :`B` 1.0 :`A` 1.0) 222.0))
        (:`Remote`
          (`KismetSystemLibrary.PrintString` "c" true true (struct :`G` 0.66 :`B` 1.0 :`A` 1.0) 222.0))))
    (:`Is Not Valid`
      (`KismetSystemLibrary.PrintString` "Hello" true true (struct :`G` 0.66 :`B` 1.0 :`A` 1.0) 222.0))))

(event `IsShoot`
  (params (NewParam :type Boolean))
  (bind _asgs_lobby (cast `/Game/GamePlay/GS_Lobby` (`GameplayStatics.GetGameState`)))
  (set `/Game/GamePlay/GS_Lobby.IsShool` NewParam _asgs_lobby))

(event `Key|One`
  (params (Key :type "Key Structure")))

(fn `Func_UI`
  (if (`self.IsLocalPlayerController`)
    (bind _returnvalue (`|CreateWidget` "/Game/UMG/UI_Lobby.UI_Lobby_C" self))
    (bind _output_get (set `self.ui` _returnvalue))
    (`UserWidget.AddToPlayerScreen` _output_get 0)
    (set `self.bShowMouseCursor` true)
    (bind _returnvalue_2 (`|CreateWidget` "/Game/UMG/UI_Login.UI_Login_C" self))
    (set `self.UiLogin` _returnvalue_2)
    (`UserWidget.AddToPlayerScreen` _returnvalue_2 1)))

(fn `UserConstructionScript`)

(fn `自定义事件`
  (params (NewParam1 :type Boolean)))